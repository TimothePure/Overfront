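; BP_OverfrontCharacter is the Overfront character Blueprint, handling the sniper scope's on-screen presentation.
; ShowSniperScopeWidget lazily creates WBP_SniperScope on first use, caches it and adds it to the viewport.
; Its ShowScope flag plays the ScopeZoomIn animation forward with a zoom-in sound, or in reverse with a zoom-out sound.
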(event `self.ShowSniperScopeWidget`
  (params (bShowScope :type Boolean))
  (bind _sniperscopewidget (`self.SniperScopeWidget`))
  (bind _sniperscopewidget_2 (`self.SniperScopeWidget`))
  (`/Engine/EditorBlueprintResources/StandardMacros.IsValid` (`self.SniperScopeWidget`)
    (:`Is Valid`
      _)
    (:`Is Not Valid`
      (bind _returnvalue (`|CreateWidget` "/Game/Overfront/Blueprints/Widgets/WBP_SniperScope.WBP_SniperScope_C"))
      (bind _output_get (set `self.SniperScopeWidget` _returnvalue))
      (`UserWidget.AddToViewport` _output_get 0)))
  (if bShowScope
    (`UserWidget.PlayAnimation` _sniperscopewidget_2 (`/Game/Overfront/Blueprints/Widgets/WBP_SniperScope.ScopeZoomIn` _sniperscopewidget_2) 0.0 1 "Forward" 1.0 false)
    (`GameplayStatics.PlaySound2D` "/Game/Assets/MilitaryWeapSilver/Sound/SniperRifle/Cues/SniperRifle_ZoomIn_Cue.SniperRifle_ZoomIn_Cue" 1.0 1.0 0.0 null null)
    (else
      (`UserWidget.PlayAnimationReverse` _sniperscopewidget (`/Game/Overfront/Blueprints/Widgets/WBP_SniperScope.ScopeZoomIn` _sniperscopewidget) 1.0 false)
      (`GameplayStatics.PlaySound2D` "/Game/Assets/MilitaryWeapSilver/Sound/SniperRifle/Cues/SniperRifle_ZoomOut_Cue.SniperRifle_ZoomOut_Cue" 1.0 1.0 0.0 null null))))

(fn `UserConstructionScript`)